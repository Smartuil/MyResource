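; GenerateBP is an actor Blueprint that builds a catalogue of video items from the project's Content/Info folder at BeginPlay.
; It scans that folder for MP4 files and uses each base name to find a matching JPG and TXT file.
; Each video becomes an item struct in ItemStructArr, holding its path, name, runtime-loaded icon texture and the text file's contents as its URL.
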(event `self.ReceiveBeginPlay`
  (bind _files (`MyBlueprintFunctionLibrary.ScanDirectory` (`KismetStringLibrary.Concat_StrStr` (`KismetSystemLibrary.GetProjectContentDirectory`) "Info/") "*.mp4"))
  (for _array_element _files
    (bind _lefts (`KismetStringLibrary.Split` _array_element "." "IgnoreCase" "FromEnd"))
    (bind _returnvalue (`MyBlueprintFunctionLibrary.CreateTextureFromFile` (`KismetStringLibrary.Concat_StrStr` _lefts ".jpg")))
    (bind _outtext (`MyBlueprintFunctionLibrary.LoadText` (`KismetStringLibrary.Concat_StrStr` _lefts ".txt")))
    (`KismetArrayLibrary.Array_Add` (`self.ItemStructArr`) (make `/Game/Struct/ItemStruct` _array_element (`.FilenamePart` (`BlueprintPathsLibrary.Split` _array_element)) _returnvalue _outtext))))

(fn `UserConstructionScript`)